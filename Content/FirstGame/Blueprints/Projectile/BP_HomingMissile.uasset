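; BP_HomingMissile is a projectile that chases the first player's pawn and explodes after five seconds or on hitting a valid pawn.
; Each Tick it smoothly turns toward the player with RInterpTo and steps forward a fixed, unswept distance per frame, so speed depends on frame rate.
; An overlap on its Cone with a pawn owning a BP_PlayerState applies damage through that state, spawns the explosion and destroys the missile.
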(event OnComponentBeginOverlap(Cone)
  (params (OverlappedComponent :type Primitive%20Component%20Object%20Reference) (OtherActor :type Actor%20Object%20Reference) (OtherComp :type Primitive%20Component%20Object%20Reference) (OtherBodyIndex :type Integer) (bFromSweep :type Boolean) (SweepResult :type Hit%20Result%20Structure%20%28by%20ref%29))
  (bind _returnvalue (Transformation|GetActorTransform))
  (bind _aspawn (Utilities|Casting|CastToPawn OtherActor))
  (bind _asbp_player_state (Utilities|Casting|CastToBP_PlayerState (Variables|/Script/Engine.Pawn|GetPlayerState _aspawn)))
  (Default|AddDamage _asbp_player_state 1e+01)
  (Effects|SpawnEmitteratLocation "/Game/StarterContent/Particles/P_Explosion.P_Explosion" (.location _returnvalue) (.rotation _returnvalue))
  (Actor|DestroyActor))

(event EventTick
  (params (DeltaSeconds :type Float%20%28single-precision%29))
  (Transformation|SetActorRotation (Math|Interpolation|RInterpTo (Transformation|GetActorRotation) (Math|Rotator|FindLookatRotation (Transformation|GetActorLocation) (Transformation|GetActorLocation (Pawn|GetControlledPawn (Game|GetPlayerController 0)))) DeltaSeconds 1e+01))
  (Transformation|AddActorWorldOffset (* (Math|Vector|GetForwardVector (Transformation|GetActorRotation)) 5.0)))

(event EventBeginPlay
  (bind _returnvalue (Transformation|GetActorTransform))
  (Utilities|FlowControl|Delay 5.0)
  (Effects|SpawnEmitteratLocation "/Game/StarterContent/Particles/P_Explosion.P_Explosion" (.location _returnvalue) (.rotation _returnvalue))
  (Actor|DestroyActor))

(fn ConstructionScript)