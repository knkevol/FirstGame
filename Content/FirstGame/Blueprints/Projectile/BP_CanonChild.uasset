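; Child cannon Blueprint that turns the parent's shot into a toggled automatic fire with limited ammo.
; PressF toggles firing: it shoots immediately, then every second on a looping timer until toggled off or out of shots.
; Each shot decrements Count, pushes it to a CountWidget display and calls the parent ShootCanon.
; Tick rotates that widget toward the player camera using only X and Y, like a yaw-only billboard.
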(event EventBeginPlay)

(event Collision|EventActorBeginOverlap
  (params (OtherActor :type Actor%20Object%20Reference))
  (|CallParentFunction OtherActor) ; This node is disabled and will not be called.\nDrag off pins to build functionality.
)

(event EventToggleCanon
  (bind _output_get (Variables|Default|SetbToggle (not (Variables|Default|GetbToggle))))
  (if _output_get
    (CallFunction|ShootCanon)
    (Utilities|Time|SetTimerbyFunctionName 0 "ShootCanon" 1.0 true)
    (else
      (Utilities|Time|ClearTimerbyFunctionName 0 "ShootCanon"))))

(event EventTick
  (params (DeltaSeconds :type Float%20%28single-precision%29))
  (CallFunction|UpdateLookCamera))

(fn ConstructionScript
  (|CallParentFunction))

(fn ReleaseF
  (params (NewParam :type Boolean))
  (return false))

(fn PressF
  (params (Character :type Character%20Object%20Reference))
  (CallFunction|ToggleCanon)
  (return false))

(fn ShootCanon
  (bind _output_get (Variables|Default|SetCount (- (Variables|Default|GetCount) 1)))
  (if (>= _output_get 0)
    (CallFunction|PrintWidget)
    (|CallParentFunction)
    (else
      (Utilities|Time|ClearTimerbyFunctionName 0 "ShootCanon"))))

(fn UpdateLookCamera
  (bind _returnvalue (Game|GetPlayerCameraManager 0))
  (bind _widget (Variables|Default|GetWidget))
  (bind _returnvalue_2 (Transformation|GetActorLocation _returnvalue))
  (bind _returnvalue_3 (Transformation|GetWorldLocation _widget))
  (Transformation|SetWorldRotation (Variables|Default|GetWidget) (Math|Rotator|FindLookatRotation (Math|Vector|MakeVector (.x _returnvalue_3) (.y _returnvalue_3) 0.0) (Math|Vector|MakeVector (.x _returnvalue_2) (.y _returnvalue_2) 0.0)) false false))

(fn PrintWidget
  (bind _ascount_widget (Utilities|Casting|CastToCountWidget (UserInterface|GetUserWidgetObject (Variables|Default|GetWidget))))
  (Default|SetCount _ascount_widget (Variables|Default|GetCount)))